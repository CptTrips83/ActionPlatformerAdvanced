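; Bat enemy that patrols endlessly back and forth between two points set by its TopPos and BottomPos components.
; At BeginPlay it caches both points in world space and sets the MoveAnim timeline's play rate from MovePlayrate.
; The timeline lerps the actor's location without sweep, and a FlipFlop on Finished alternates reverse and forward playback to sustain the loop.
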(event Custom|Move%20Forward
  (bind _alpha (Timeline|MoveAnim PlayFromStart)
    (:Update
      (Transformation|SetActorLocation (Math|Vector|Lerp(Vector) (Variables|Default|GetWorldTopPosition) (Variables|Default|GetWorldBottomPosition) _alpha) false false))
    (:Finished
      (Utilities|FlowControl|FlipFlop
        (:A
          (CallFunction|MoveBackward))
        (:B
          (CallFunction|MoveForward))))))

(event Custom|Move%20Backward
  (bind _alpha (Timeline|MoveAnim ReverseFromEnd)
    (:Update
      (Transformation|SetActorLocation (Math|Vector|Lerp(Vector) (Variables|Default|GetWorldTopPosition) (Variables|Default|GetWorldBottomPosition) _alpha) false false))
    (:Finished
      (Utilities|FlowControl|FlipFlop
        (:A
          (CallFunction|MoveBackward))
        (:B
          (CallFunction|MoveForward))))))

(event EventBeginPlay
  (|CallParentFunction)
  (Variables|Default|SetWorldTopPosition (Transformation|GetWorldLocation (Variables|Default|GetTopPos)))
  (Variables|Default|SetWorldBottomPosition (Transformation|GetWorldLocation (Variables|Default|GetBottomPos)))
  (Components|Timeline|SetPlayRate (Variables|Default|GetMoveAnim) (Variables|Default|GetMove%20Playrate))
  (CallFunction|MoveForward))

(event Collision|EventActorBeginOverlap
  (params (OtherActor :type Actor%20Object%20Reference))
  (|CallParentFunction OtherActor) ; This node is disabled and will not be called.\nDrag off pins to build functionality.
)

(event EventTick
  (params (DeltaSeconds :type Float%20%28single-precision%29))
  (|CallParentFunction DeltaSeconds) ; This node is disabled and will not be called.\nDrag off pins to build functionality.
)

(fn ConstructionScript
  (|CallParentFunction))