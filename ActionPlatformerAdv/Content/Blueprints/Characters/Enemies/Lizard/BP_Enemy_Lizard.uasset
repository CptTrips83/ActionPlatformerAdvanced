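; Lizard enemy Blueprint that attacks by shooting fireballs.
; ShootFireball clears current animation overrides on the animation component's instance and plays the Shoot sequence as an override.
; SpawnProjectile separately spawns a lizard projectile actor at the ShootPosition component's location and rotation, regardless of collision.
; The event graph holds only disabled default events, and nothing in this Blueprint calls either function.
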(event EventBeginPlay
  (|CallParentFunction) ; This node is disabled and will not be called.\nDrag off pins to build functionality.
)

(event Collision|EventActorBeginOverlap
  (params (OtherActor :type Actor%20Object%20Reference))
  (|CallParentFunction OtherActor) ; This node is disabled and will not be called.\nDrag off pins to build functionality.
)

(event EventTick
  (params (DeltaSeconds :type Float%20%28single-precision%29))
  (|CallParentFunction DeltaSeconds) ; This node is disabled and will not be called.\nDrag off pins to build functionality.
)

(fn ConstructionScript
  (|CallParentFunction))

(fn ShootFireball
  (bind _animationcomponent (Variables|Default|GetAnimationComponent))
  (bind _animinstance (Variables|/Script/PaperZD.PaperZDAnimationComponent|GetAnimInstance _animationcomponent))
  (Class|PaperZDAnimInstance|StopAllAnimationOverrides _animinstance)
  (Class|PaperZDAnimInstance|PlayAnimationOverride _animinstance "/Game/Blueprints/Characters/Enemies/Lizard/AnimSequences/Shoot.Shoot" "DefaultSlot" 1.0 0.0))

(fn SpawnProjectile
  (bind _shootposition (Variables|Default|GetShootPosition))
  (bind _returnvalue (Transformation|GetWorldTransform _shootposition))
  (Game|SpawnActorfromClass "/Game/Blueprints/Projectiles/Enemy/BP_EnemyProjectile_Lizard.BP_EnemyProjectile_Lizard_C" (Math|Transform|MakeTransform (.location _returnvalue) (.rotation _returnvalue) "1.000000,1.000000,1.000000") "AlwaysSpawn" "MultiplyWithRoot" 0 0))