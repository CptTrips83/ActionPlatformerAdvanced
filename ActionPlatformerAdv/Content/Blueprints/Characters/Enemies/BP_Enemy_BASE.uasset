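; BP_Enemy_BASE is, by its name, the base Blueprint for enemies, providing a visual effect when one is destroyed.
; On Destroyed, it spawns BP_VFX_EnemyDestroyed at the actor's current location and rotation.
; BeginPlay, overlap and Tick are disabled placeholders, and the construction script only calls its parent.
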(event EventBeginPlay
  (|CallParentFunction) ; This node is disabled and will not be called.\nDrag off pins to build functionality.
)

(event Collision|EventActorBeginOverlap
  (params (OtherActor :type Actor%20Object%20Reference))
  (|CallParentFunction OtherActor) ; This node is disabled and will not be called.\nDrag off pins to build functionality.
)

(event EventTick
  (params (DeltaSeconds :type Float%20%28single-precision%29))
  (|CallParentFunction DeltaSeconds) ; This node is disabled and will not be called.\nDrag off pins to build functionality.
)

(event EventDestroyed
  (Game|SpawnActorfromClass "/Game/Blueprints/VFX/BP_VFX_EnemyDestroyed.BP_VFX_EnemyDestroyed_C" (Math|Transform|MakeTransform (Transformation|GetActorLocation) (Transformation|GetActorRotation) "1.000000,1.000000,1.000000") "Undefined" "MultiplyWithRoot" 0 0))

(fn ConstructionScript
  (|CallParentFunction))