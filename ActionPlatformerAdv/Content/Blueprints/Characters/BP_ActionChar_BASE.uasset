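; BP_ActionChar_BASE is a base action character Blueprint that handles taking damage and flashing its sprite when hit.
; AnyDamage feeds the Vitality component, then destroys the actor if defeated or triggers an orange flash otherwise.
; TriggerFlash drives a dynamic sprite material created at BeginPlay and plays the FadeSpriteFlash timeline, whose lerp toward zero is applied only on Finished, not per update.
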(event Custom|TriggerFlash
  (params (FlashMultiplier :type Float%20%28single-precision%29) (FlashColor :type Linear%20Color%20Structure))
  (Rendering|Material|SetScalarParameterValue (Variables|Default|GetDynamicSpriteMat) "FlashMultiplier" FlashMultiplier :!class /Script/Engine.MaterialInstanceDynamic)
  (Rendering|Material|SetVectorParameterValue (Variables|Default|GetDynamicSpriteMat) "FlashColor" FlashColor :!class /Script/Engine.MaterialInstanceDynamic)
  (Components|Timeline|SetPlayRate (Variables|Default|GetFadeSpriteFlash) (Variables|Default|GetSpriteFlashPlayRate))
  (bind _alpha (Timeline|FadeSpriteFlash PlayFromStart)
    (:Finished
      (Rendering|Material|SetScalarParameterValue (Variables|Default|GetDynamicSpriteMat) "FlashMultiplier" (Math|Float|Lerp FlashMultiplier 0.0 _alpha) :!class /Script/Engine.MaterialInstanceDynamic))))

(event Game|Damage|EventAnyDamage
  (params (Damage :type Float%20%28single-precision%29) (DamageType :type Damage%20Type%20Object%20Reference) (InstigatedBy :type Controller%20Object%20Reference) (DamageCauser :type Actor%20Object%20Reference))
  (Default|ReceiveDamage (Variables|Default|GetVitality) Damage)
  (if (Variables|/Game/Blueprints/Components/BPC_Vitality.BPC_Vitality_C|GetIsDefeated (Variables|Default|GetVitality))
    (Actor|DestroyActor)
    (else
      (CallFunction|TriggerFlash 1e+01 "(R=1.000000,G=0.575578,B=0.000000,A=1.000000)"))))

(event EventBeginPlay
  (bind _returnvalue (Rendering|Material|CreateDynamicMaterialInstance (Variables|Default|GetSprite) 0 0 "None" :!class /Script/Engine.PrimitiveComponent))
  (Variables|Default|SetDynamicSpriteMat _returnvalue))

(fn ConstructionScript)