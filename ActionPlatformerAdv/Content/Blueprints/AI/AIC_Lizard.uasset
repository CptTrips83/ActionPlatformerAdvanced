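; AI controller for the lizard enemy that makes it shoot fireballs at a regular interval.
; On possess, it caches the pawn as BP_Enemy_Lizard and starts a looping timer based on ShootInterval.
; The ShootProjectile event, evidently the timer's callback, delegates the shot to the lizard's ShootFireball, with no targeting or movement logic in the controller.
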(event Custom|ShootProjectile
  (Default|ShootFireball (Variables|Default|GetOwningLizard)))

(event EventPossess
  (params (PossessedPawn :type Pawn%20Object%20Reference))
  (|CallParentFunction PossessedPawn)
  (bind _asbp_enemy_lizard (Utilities|Casting|CastToBP_Enemy_Lizard PossessedPawn))
  (Variables|Default|SetOwningLizard _asbp_enemy_lizard)
  (Utilities|Time|SetTimerbyEvent (EventDispatchers|CreateEvent :!event Custom|ShootProjectile) (Variables|Default|GetShootInterval) true))

(fn ConstructionScript
  (|CallParentFunction))