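; AIC_Eye is the AI controller for the BP_Enemy_Eye enemy, steering it toward a target pawn.
; On possession it caches the controlled eye, and SetTargetPlayer stores the pawn to chase.
; Every tick it calls the eye's MoveTowards at full scale along the direct look-at direction to the target, using no pathfinding or behavior tree.
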(event Custom|Set%20Target%20Player
  (params (Target%20Pawn :type Pawn%20Object%20Reference))
  (Variables|Default|SetTarget%20Pawn Target%20Pawn))

(event EventPossess
  (params (PossessedPawn :type Pawn%20Object%20Reference))
  (bind _asbp_enemy_eye (Utilities|Casting|CastToBP_Enemy_Eye PossessedPawn))
  (Variables|Default|SetOwning%20Eye _asbp_enemy_eye))

(event EventTick
  (params (DeltaSeconds :type Float%20%28single-precision%29))
  (Variables|Default|GetOwning%20Eye
    (:then
      (Variables|Default|GetTarget%20Pawn
        (:then
          (Default|MoveTowards (Variables|Default|GetOwning%20Eye) (Math|Vector|GetForwardVector (Math|Rotator|FindLookatRotation (Transformation|GetActorLocation (Variables|Default|GetOwning%20Eye)) (Transformation|GetActorLocation (Variables|Default|GetTarget%20Pawn)))) 1.0))
        (:else)))
    (:else)))

(fn ConstructionScript
  (|CallParentFunction))